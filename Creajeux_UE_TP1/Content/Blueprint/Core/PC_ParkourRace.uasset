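; PC_ParkourRace is the player controller for the parkour race, handling input setup and the pause action.
; On BeginPlay it adds the third-person Enhanced Input mapping context, caches the HUD_ParkourRace instance and sets game-only input mode.
; The IA_Pause action calls PauseMode on that HUD, and does not fire while the controller is in UI-only input mode.
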(event `self.ReceiveBeginPlay`
  (bind _returnvalue (subsystem `EnhancedInputLocalPlayerSubsystem`))
  (`/Engine/EditorBlueprintResources/StandardMacros.IsValid` _returnvalue
    (:`Is Valid`
      (`EnhancedInputSubsystemInterface.AddMappingContext` _returnvalue "/Game/Blueprint/Input/IMC_ThirdPerson.IMC_ThirdPerson" 0 (struct))
      (bind _ashud_parkour_race (cast `/Game/Blueprint/Core/HUD_ParkourRace` (`self.GetHUD`)))
      (set `self.HUD Parkour Race` _ashud_parkour_race)
      (`WidgetBlueprintLibrary.SetInputMode_GameOnly` (`GameplayStatics.GetPlayerController` 0)))))

(event `EnhancedInput|/Game/Blueprint/Input/IA_Pause`
  (params (ActionValue :type Boolean) (ElapsedSeconds :type "Float (double-precision)") (TriggeredSeconds :type "Float (double-precision)") (InputAction :type "InputAction Object Reference" :default "/Game/Blueprint/Input/IA_Pause.IA_Pause"))
  (:`Started`
    (`/Game/Blueprint/Core/HUD_ParkourRace.PauseMode` (`self.HUD Parkour Race`))))

(fn `UserConstructionScript`)