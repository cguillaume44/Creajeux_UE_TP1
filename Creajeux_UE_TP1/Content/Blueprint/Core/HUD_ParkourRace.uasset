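; HUD class for the parkour race that creates the W_HUDWidget on BeginPlay, adds it to the viewport and plays its match start animation.
; PauseMode and GameMode switch the widget switcher between gameplay and pause views, toggling input mode, mouse cursor and game pause together.
; The widget receives a reference to this HUD on creation and is stored in a variable to protect it from garbage collection.
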(event `self.ReceiveBeginPlay`
  (bind _returnvalue (`|CreateWidget` "/Game/Blueprint/UI/W_HUDWidget.W_HUDWidget_C" (`GameplayStatics.GetPlayerController` 0) self))
  (bind _output_get (set `self.HUDWidget` _returnvalue)) ; Promote to variable\nSaved from garbage collection!
  (`UserWidget.AddToViewport` _output_get 0)
  (`/Game/Blueprint/UI/W_HUDWidget.PlayAnim` _output_get (`/Game/Blueprint/UI/W_HUDWidget.MatchStartAnim` _output_get) 1.0))

(fn `GameMode`
  (bind _returnvalue (`GameplayStatics.GetPlayerController` 0))
  (set `WidgetSwitcher.ActiveWidgetIndex` 0 (`/Game/Blueprint/UI/W_HUDWidget.HUDSwitcher` (`self.HUDWidget`)))
  (`WidgetBlueprintLibrary.SetInputMode_GameOnly` _returnvalue)
  (set `PlayerController.bShowMouseCursor` false _returnvalue)
  (`GameplayStatics.SetGamePaused` false))

(fn `PauseMode`
  (bind _returnvalue (`GameplayStatics.GetPlayerController` 0))
  (set `WidgetSwitcher.ActiveWidgetIndex` 1 (`/Game/Blueprint/UI/W_HUDWidget.HUDSwitcher` (`self.HUDWidget`)))
  (`WidgetBlueprintLibrary.SetInputMode_UIOnlyEx` _returnvalue null)
  (set `PlayerController.bShowMouseCursor` true _returnvalue)
  (`GameplayStatics.SetGamePaused` true))

(fn `UserConstructionScript`)