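; GM_ParkourRace is the game mode for the parkour race, handling checkpoints, respawning and winning.
; It stores the current checkpoint, and RespawnChara spawns and possesses a new P_MainChara there, falling back to a PlayerStart lookup that is flagged as unsafe.
; Win plays the HUD's match-over animation, then loads the main menu level when it finishes.
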(event `self.ReceiveBeginPlay`)

(event `/Game/Blueprint/Core/BPI_Player.UpdateCheckpoint`
  (params (NewCheckpoint :type "/Game/Blueprint/Actors/BP_Checkpoint Object Reference"))
  (set `self.CurrentCheckpoint` NewCheckpoint))

(event `/Game/Blueprint/Core/BPI_Player.Win`
  (bind _ashud_parkour_race (cast `/Game/Blueprint/Core/HUD_ParkourRace` (`PlayerController.GetHUD` (`GameplayStatics.GetPlayerController` 0))))
  (bind _hudwidget (`/Game/Blueprint/Core/HUD_ParkourRace.HUDWidget` _ashud_parkour_race))
  (bind _matchoveranim (`/Game/Blueprint/UI/W_HUDWidget.MatchOverAnim` _hudwidget))
  (`/Game/Blueprint/UI/W_HUDWidget.PlayAnim` _hudwidget _matchoveranim 1.0)
  (`UserWidget.BindToAnimationFinished` _hudwidget _matchoveranim (delegate `Load`)))

(event `Load`
  (`GameplayStatics.OpenLevelBySoftObjectPtr` "/Game/Levels/L_MainMenu.L_MainMenu"))

(fn `RespawnChara`
  (locals (SpawnTansform :type "Transform Structure"))
  ;[1 1 1] GM_ParkourRace
  (`/Engine/EditorBlueprintResources/StandardMacros.IsValid` (`self.CurrentCheckpoint`)
    (:`Is Valid`
      (set `local.SpawnTansform` (`SceneComponent.K2_GetComponentToWorld` (`/Game/Blueprint/Actors/BP_Checkpoint.SpawnLoc` (`self.CurrentCheckpoint`)))))
    (:`Is Not Valid`
      (bind _returnvalue (`GameplayStatics.GetActorOfClass` "/Script/Engine.PlayerStart")) ; Not safe at all! \nThis must be changed when we have\nthe checkpoint system!
      (`/Engine/EditorBlueprintResources/StandardMacros.IsValid` _returnvalue
        (:`Is Valid`
          (set `local.SpawnTansform` (`self.GetTransform` _returnvalue)))
        (:`Is Not Valid`
          (`KismetSystemLibrary.PrintString` "No player start found!" true true (struct :`R` 1.0 :`G` 0.022436 :`A` 1.0) 5.0)
          (return)))))
  (bind _returnvalue_2 (`|SpawnActorFromClass` "/Game/Blueprint/P_MainChara.P_MainChara_C" (`local.SpawnTansform`) "AlwaysSpawn" "MultiplyWithRoot" null null))
  (`Controller.Possess` (`GameplayStatics.GetPlayerController` 0) _returnvalue_2)
  (return))

(fn `UserConstructionScript`)