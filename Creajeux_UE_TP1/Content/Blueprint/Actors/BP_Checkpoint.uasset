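; BP_Checkpoint is a checkpoint actor that notifies the game mode when something enters its Box trigger.
; The overlap sends an UpdateCheckpointMessage interface call to the game mode with itself as the argument, without filtering the overlapping actor.
; The construction script gives the Plane a dynamic instance of MI_Checkpoint, driven by the actor's PannerSpeed and Color variables for scroll speed and tint.
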(event `self.Box.OnComponentBeginOverlap`
  (params (OverlappedComponent :type "PrimitiveComponent Object Reference") (OtherActor :type "Actor Object Reference") (OtherComp :type "PrimitiveComponent Object Reference") (OtherBodyIndex :type Integer) (bFromSweep :type Boolean) (SweepResult :type "HitResult Structure (by ref)"))
  ;[1 1 1] Checkpoint
  (message `/Game/Blueprint/Core/BPI_Player.UpdateCheckpoint` (`GameplayStatics.GetGameMode`) self) ; BPI message
)

(fn `UserConstructionScript`
  (bind (_pannerspeed_x _pannerspeed_y) (`KismetMathLibrary.BreakVector2D` (`self.PannerSpeed`)))
  (bind _returnvalue (`PrimitiveComponent.CreateDynamicMaterialInstance` (`self.Plane`) 0 "/Game/Material/MI_Checkpoint.MI_Checkpoint" "None"))
  (`PrimitiveComponent.SetMaterial` (`self.Plane`) 0 _returnvalue)
  (`MaterialInstanceDynamic.SetScalarParameterValue` _returnvalue "SpeedX" _pannerspeed_x)
  (`MaterialInstanceDynamic.SetScalarParameterValue` _returnvalue "SpeedY" _pannerspeed_y)
  (`MaterialInstanceDynamic.SetVectorParameterValue` _returnvalue "Color" (`self.Color`)))