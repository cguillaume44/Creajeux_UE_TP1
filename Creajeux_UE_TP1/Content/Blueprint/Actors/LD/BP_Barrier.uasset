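; BP_Barrier is a level-design barrier actor that builds a row of border pillars and beams along a spline.
; The construction script loops over every spline point, adding a pillar static mesh there and a spline mesh beam to the next point, shaped by both points' tangents.
; The last point gets no special handling and still adds a beam toward a following index.
; The event graph has no active logic.
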(fn `UserConstructionScript`
  (bind _spline (`self.Spline`))
  (for _index (range (`SplineComponent.GetNumberOfSplinePoints` (`self.Spline`)))
    (bind _returnvalue (`AddComponent|NODE_AddStaticMeshComponent-0`)) ; SM_Border_Pillar in details panel
    (`SceneComponent.K2_SetRelativeLocation` _returnvalue (`SplineComponent.GetLocationAtSplinePoint` (`self.Spline`) _index "Local") false false)
    (bind _returnvalue_2 (`AddComponent|NODE_AddSplineMeshComponent-1`)) ; SM_Border_Beams in details panel
    (bind (_location _tangent) (`SplineComponent.GetLocationAndTangentAtSplinePoint` _spline _index "Local"))
    (bind (_location_2 _tangent_2) (`SplineComponent.GetLocationAndTangentAtSplinePoint` _spline (+ _index 1) "Local"))
    (`SplineMeshComponent.SetStartAndEnd` _returnvalue_2 _location _tangent _location_2 _tangent_2 true)))