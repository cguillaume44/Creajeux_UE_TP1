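; BP_Bumper is a jump pad actor that bumps the player when something hits its mesh.
; On hit, it checks that the other actor implements BPI_Player, then sends BumpPlayerMessage with the Arrow component's forward vector and a Strenght value.
; The same hit restarts a Timeline whose Height track overrides the pad's world Z scale for a squash/stretch animation, so non-player hits trigger neither bump nor animation.
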(event `self.SM_Jump_Pad.OnComponentHit`
  (params (HitComponent :type "PrimitiveComponent Object Reference") (OtherActor :type "Actor Object Reference") (OtherComp :type "PrimitiveComponent Object Reference") (NormalImpulse :type "Vector Structure") (Hit :type "HitResult Structure (by ref)"))
  (bind (_returnvalue_x _returnvalue_y) (`KismetMathLibrary.BreakVector` (`SceneComponent.K2_GetComponentScale` (`self.SM_Jump_Pad`))))
  (if (`KismetSystemLibrary.DoesImplementInterface` OtherActor "/Game/Blueprint/Core/BPI_Player.BPI_Player_C")
    (message `/Game/Blueprint/Core/BPI_Player.BumpPlayer` OtherActor (`SceneComponent.GetForwardVector` (`self.Arrow`)) (`self.Strenght`)) ; BPI call!
    (bind (_direction _height) (`Timeline|Timeline` :!via `PlayFromStart`) ; Ideally save the original Z scale \nand apply a multiply factor to it.
      (:`Update`
        (`SceneComponent.SetWorldScale3D` (`self.SM_Jump_Pad`) (`KismetMathLibrary.MakeVector` _returnvalue_x _returnvalue_y _height))))))

(fn `UserConstructionScript`)