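; BP_MasterGActor is an actor Blueprint, apparently a base for timeline-animated objects, with helpers to move and rotate a ToAnimate component.
; On BeginPlay it starts every timeline component at a random time and applies a shared play rate, so instances animate out of sync.
; Translate lerps ToAnimate's relative location between the PosA and PosB markers by Alpha, and Rotate sets its relative rotation directly.
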(event `self.ReceiveBeginPlay`
  (for _array_element (`self.K2_GetComponentsByClass` "/Script/Engine.TimelineComponent")
    (`TimelineComponent.SetNewTime` _array_element (`KismetMathLibrary.RandomFloatInRange` 0.0 (`TimelineComponent.GetTimelineLength` _array_element)))
    (`TimelineComponent.SetPlayRate` _array_element (`self.New Rate`))))

(fn `Rotate`
  (params (`New Rotation X (Roll)` :type "Float (single-precision)") (`New Rotation Y (Pitch)` :type "Float (single-precision)") (`New Rotation Z (Yaw)` :type "Float (single-precision)"))
  (`SceneComponent.K2_SetRelativeRotation` (`self.ToAnimate`) (`KismetMathLibrary.MakeRotator` `New Rotation X (Roll)` `New Rotation Y (Pitch)` `New Rotation Z (Yaw)`) false false)
  (return))

(fn `Translate`
  (params (Alpha :type "Float (single-precision)"))
  (`SceneComponent.K2_SetRelativeLocation` (`self.ToAnimate`) (`KismetMathLibrary.VLerp` (`SceneComponent.RelativeLocation` (`self.PosA`)) (`SceneComponent.RelativeLocation` (`self.PosB`)) Alpha) false false)
  (return))

(fn `UserConstructionScript`)